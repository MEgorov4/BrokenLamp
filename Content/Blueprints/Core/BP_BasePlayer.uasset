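; Base player character with axis-flippable movement, interaction, footstep audio and reaction text.
; Each tick it caches the closest overlapping BP_InteractableActor that allows interaction, and press, hold and tap inputs are forwarded to that actor.
; Tick also accumulates horizontal distance to trigger steps, playing a snow sound, then a line trace can switch it by surface type.
; A gate blocks new reactions until the widget finishes typing and hides after a delay.
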(event `self.ReceiveBeginPlay`
  ; Ebani` costil
  (`SceneComponent.SetVisibility` (`self.Widget`) false false))

(event `self.ReceiveTick`
  (params (DeltaSeconds :type "Float (single-precision)"))
  (`|ExecutionSequence`
    (:`then_0`
      (`self.ProcessInteractableActors`))
    (:`then_1`
      (`self.ProcessSteps`))))

(event `ProcessInteractableActors`
  ; Process Interaction Actors
  (bind _focusedinteractableactor (`self.FillAllInteractableActorsWithTrueCanInteract`))
  (bind _interactableactor (`self.GetClosestInteractableActor` _focusedinteractableactor))
  (`/Engine/EditorBlueprintResources/StandardMacros.IsValid` _interactableactor
    (:`Is Valid`
      (set `self.PossibleInteractableActor` _interactableactor))))

(event `ShowReaction`
  (params (ReactionText :type Text))
  ; Character Reaction Logic
  (`/Engine/EditorBlueprintResources/StandardMacros.Gate` false :!label _label
    (:`Exit`
      (bind _asbpw_character_reaction_widget (cast `/Game/Blueprints/Widgets/Characters/BPW_CharacterReactionWidget` (`WidgetComponent.GetWidget` (`self.Widget`))))
      (add `/Game/Blueprints/Widgets/Characters/BPW_CharacterReactionWidget.TypingComplete` _asbpw_character_reaction_widget (`|CreateDelegate` :!event `TypingReactionComplete`))
      (`/Game/Blueprints/Widgets/Characters/BPW_CharacterReactionWidget.SetReactionText` _asbpw_character_reaction_widget ReactionText)
      (`SceneComponent.SetVisibility` (`self.Widget`) true false)
      (goto _label :!via `Close`))))

(event `TypingReactionComplete`
  ; Character Reaction Logic
  (`KismetSystemLibrary.Delay` (`self.ShowReactionDuration`))
  (`SceneComponent.SetVisibility` (`self.Widget`) false false)
  (goto _label :!via `Open`))

(fn `GetClosestInteractableActor`
  (params (Actors :type "Array of /Game/Blueprints/Interaction/BP_InteractableActor Object Reference"))
  (returns (InteractableActor :type "/Game/Blueprints/Interaction/BP_InteractableActor Object Reference"))
  (locals (Distance :type "Float (double-precision)" :default 1000.0) (CurentClosest :type "/Game/Blueprints/Interaction/BP_InteractableActor Object Reference"))
  (set `local.Distance` 1000.0)
  (for _array_element Actors
    (bind _returnvalue (`self.GetDistanceTo` _array_element self))
    (if (< _returnvalue (`local.Distance`))
      (set `local.Distance` _returnvalue)
      (set `local.CurentClosest` _array_element)))
  (return (`local.CurentClosest`)))

(fn `HoldInteract`
  (bind _possibleinteractableactor (`self.PossibleInteractableActor`))
  (`/Engine/EditorBlueprintResources/StandardMacros.IsValid` _possibleinteractableactor
    (:`Is Valid`
      (message `/Game/Blueprints/Interaction/BPI_Interactable.HoldInteract` _possibleinteractableactor self)
      (return))))

(fn `Move`
  (params (Direction :type "Vector2D Structure"))
  (if (`self.bIsReversed`)
    (`self.AddMovementInput` (`KismetMathLibrary.MakeVector` Direction_Y Direction_X))
    (return)
    (else
      (`self.AddMovementInput` (`KismetMathLibrary.MakeVector` (* Direction_X -1.0) Direction_Y))
      (return))))

(fn `PressInteract`
  (bind _possibleinteractableactor (`self.PossibleInteractableActor`))
  (`/Engine/EditorBlueprintResources/StandardMacros.IsValid` _possibleinteractableactor
    (:`Is Valid`
      (message `/Game/Blueprints/Interaction/BPI_Interactable.PressInteract` _possibleinteractableactor self)
      (return))))

(fn `SelectCurrentInteraction`
  (returns (InteractableActor :type "/Game/Blueprints/Interaction/BP_InteractableActor Object Reference"))
  (`self.FillAllInteractableActorsWithTrueCanInteract`))

(fn `TapInteract`
  (bind _possibleinteractableactor (`self.PossibleInteractableActor`))
  (`/Engine/EditorBlueprintResources/StandardMacros.IsValid` _possibleinteractableactor
    (:`Is Valid`
      (message `/Game/Blueprints/Interaction/BPI_Interactable.TapInteract` _possibleinteractableactor self)
      (return))))

(fn `UserConstructionScript`)