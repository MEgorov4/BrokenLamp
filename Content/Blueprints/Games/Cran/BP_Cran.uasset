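; Player-operated crane that moves by up and right offsets and picks up or drops BP_InteractableActor cargo.
; Offset changes trigger a swept move from the start position, blocked when a box trace sized to the carried cargo hits, with hit state broadcast every Tick.
; Interact uses downward line traces to attach cargo or release it near a surface, switching its collision object type.
; Player overlaps set the interaction prompt widget by character.
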(event `OnActorHit_Event` :!signature `self.OnActorHit`
  (params (SelfActor :type "Actor Object Reference") (OtherActor :type "Actor Object Reference") (NormalImpulse :type "Vector Structure") (Hit :type "HitResult Structure (by ref)")))

(event `self.ReceiveBeginPlay`
  (set `self.InitialLocaiton` (`SceneComponent.K2_GetComponentLocation` (`self.StaticMesh`)))
  (`PrimitiveComponent.SetCollisionEnabled` (`self.StaticMesh`) "QueryAndPhysics")
  (add `self.UpdateLocation` (delegate `UpdateLocation_Event`))
  (add `self.OnActorHit` (delegate `OnActorHit_Event`)))

(event `UpdateLocation_Event`
  (bind _cargoactor (`self.CargoActor`))
  (bind _returnvalue (+ (`self.InitialCargoLocation`) (- (`self.UpOffset`) (`self.UpCargoOffsetCut`)) (- (`self.RightOffset`) (`self.RightCargoOffsetCut`))))
  (if (`KismetSystemLibrary.IsValid` _cargoactor)
    (bind (_outhit _returnvalue_2) (`KismetSystemLibrary.BoxTraceSingle` _returnvalue _returnvalue (`.BoxExtent` (`KismetSystemLibrary.GetComponentBounds` (`/Game/Blueprints/Interaction/BP_InteractableActor.StaticMesh` _cargoactor))) (struct) "TraceTypeQuery1" false (`|MakeArray` self (`self.CargoActor`) :!type "Actor Object Reference") "ForDuration" true (struct :`R` 1.0 :`A` 1.0) (struct :`G` 1.0 :`A` 1.0) 0.0))
    (`KismetSystemLibrary.PrintString` (`KismetSystemLibrary.GetDisplayName` (`.HitActor` (`GameplayStatics.BreakHitResult` _outhit))))
    (if _returnvalue_2
      (set `self.bLastHit` true)
      (else
        (bind _sweephitresult (`self.K2_SetActorLocation` (+ (`self.InitialLocaiton`) (`self.UpOffset`) (`self.RightOffset`)) true :!label _label))
        (`|ExecutionSequence`
          (:`then_0`
            (set `self.bLastHit` (`GameplayStatics.BreakHitResult` _sweephitresult))
            (if (`self.bCargoHit`)
              (set `self.bLastHit` false)))
          (:`then_1`
            (if (== (`self.UpOffset`) (0.0 0.0 0.0))
              (set `self.bUpNow` true)
              (else
                (set `self.bUpNow` false))))
          (:`then_2`
            (if (== (`self.RightOffset`) (0.0 0.0 0.0))
              (set `self.bRigthNow` true)
              (else
                (set `self.bRigthNow` false)))))))
    (else
      (goto _label))))

(event `self.ReceiveTick`
  (params (DeltaSeconds :type "Float (single-precision)"))
  (`parent.ReceiveTick` DeltaSeconds)
  (`self.OnHitDetected` (`self.bLastHit`)))

(event `/Game/Blueprints/Interaction/BPI_Interactable.PressInteract`
  (params (InvistigaterCharacter :type "/Game/Blueprints/Core/BP_BasePlayer Object Reference"))
  (bind _returnvalue (`SceneComponent.K2_GetComponentLocation` (`self.Cargo`)))
  (bind _returnvalue_2 (`SceneComponent.K2_GetComponentLocation` (`self.Cargo`)))
  (bind (_origin _boxextent) (`KismetSystemLibrary.GetComponentBounds` (`/Game/Blueprints/Interaction/BP_InteractableActor.StaticMesh` (`self.CargoActor`))))
  (bind _returnvalue_3 (`KismetMathLibrary.MakeVector` (.x _origin) (.y _origin) (- (.z _origin) (.z _boxextent))))
  (bind _return (`self.CheckCanInteract`))
  (if _return
    (bind _outhits (`KismetSystemLibrary.LineTraceMulti` :`Start` _returnvalue_2 :`End` (+ _returnvalue_2 (* (`SceneComponent.GetUpVector` (`self.Cargo`)) -20.0)) :`TraceChannel` "TraceTypeQuery1" :`DrawDebugType` "ForDuration"))
    (for _array_element _outhits
      (if (`KismetSystemLibrary.IsValid` (`self.CargoActor`))
        (bind _outhits_2 (`KismetSystemLibrary.LineTraceMulti` _returnvalue (+ _returnvalue (* (`SceneComponent.GetUpVector` (`self.Cargo`)) -200.0)) "TraceTypeQuery1" false (`|MakeArray` (`self.CargoActor`) :!type "Actor Object Reference") "ForDuration"))
        (for _array_element_2 _outhits_2
          (if (< (`.Distance` (`GameplayStatics.BreakHitResult` _array_element_2)) 100.0)
            (`/Engine/EditorBlueprintResources/StandardMacros.IsValid` (`self.CargoActor`)
              (:`Is Valid`
                (`self.K2_DetachFromActor` (`self.CargoActor`) "KeepWorld" "KeepWorld" "KeepWorld")
                (`PrimitiveComponent.SetCollisionObjectType` (`/Game/Blueprints/Interaction/BP_InteractableActor.StaticMesh` (`self.CargoActor`)) "ECC_GameTraceChannel1")
                (set `/Game/Blueprints/Interaction/BP_InteractableActor.bCompleted` false (`self.CargoActor`))
                (set `self.CargoActor` null)))))
        (else
          (bind _asbp_interactable_actor (cast `/Game/Blueprints/Interaction/BP_InteractableActor` (`.HitActor` (`GameplayStatics.BreakHitResult` _array_element))))
          (`self.K2_AttachToComponent` _asbp_interactable_actor (`self.Cargo`) "None" "KeepWorld" "KeepWorld" "KeepWorld" true)
          (bind _output_get (set `self.CargoActor` _asbp_interactable_actor))
          (`PrimitiveComponent.SetCollisionObjectType` (`/Game/Blueprints/Interaction/BP_InteractableActor.StaticMesh` _output_get) "ECC_GameTraceChannel3")
          (set `self.InitialCargoLocation` (`SceneComponent.K2_GetComponentLocation` (`/Game/Blueprints/Interaction/BP_InteractableActor.StaticMesh` (`self.CargoActor`))))
          (set `self.UpCargoOffsetCut` (`self.UpOffset`))
          (set `self.RightCargoOffsetCut` (`self.RightOffset`))
          (set `self.BottomOfCargo` _returnvalue_3)
          (set `/Game/Blueprints/Interaction/BP_InteractableActor.bCompleted` true (`self.CargoActor`))
          (`KismetSystemLibrary.PrintString` (`KismetStringLibrary.Conv_VectorToString` _returnvalue_3) true true (struct :`R` 1.0 :`G` 0.792413 :`A` 1.0) 10.0))))))

(event `self.InteractableArea.OnComponentBeginOverlap`
  (params (OverlappedComponent :type "PrimitiveComponent Object Reference") (OtherActor :type "Actor Object Reference") (OtherComp :type "PrimitiveComponent Object Reference") (OtherBodyIndex :type Integer) (bFromSweep :type Boolean) (SweepResult :type "HitResult Structure (by ref)"))
  (bind (_actorinteractioninfo_interactiontype _actorinteractioninfo_interactionsocialtype) (break `/Game/Blueprints/Interaction/S_ObjectInteractionInfo` (`self.ActorInteractionInfo`)))
  (bind _asbp_base_player (cast `/Game/Blueprints/Core/BP_BasePlayer` OtherActor))
  (`KismetArrayLibrary.Array_AddUnique` (`self.InteractableActors`) _asbp_base_player)
  (if (>= (`KismetArrayLibrary.Array_Length` (`self.InteractableActors`)) 1) :!label _label_2
    (cast `/Game/Blueprints/Core/BP_Anna` (`|GetArrayItem` (`self.InteractableActors`))
      (:`then`
        (set `self.ActorInteractionInfo` (make `/Game/Blueprints/Interaction/S_ObjectInteractionInfo` "NewEnumerator2")))
      (:`CastFailed`
        (set `self.ActorInteractionInfo` (make `/Game/Blueprints/Interaction/S_ObjectInteractionInfo` "NewEnumerator2" "NewEnumerator1"))))
    (bind _asbpw_interaction_type_widget (cast `/Game/Blueprints/Widgets/Actors/BPW_InteractionTypeWidget` (`WidgetComponent.GetWidget` (`self.Widget`))))
    (`/Game/Blueprints/Widgets/Actors/BPW_InteractionTypeWidget.SetType` _asbpw_interaction_type_widget _actorinteractioninfo_interactiontype _actorinteractioninfo_interactionsocialtype)
    (set `/Game/Blueprints/Interaction/ActionHandlers/BP_HoldInteractionHandler.InteractionSocialType` "NewEnumerator0" (`self.BP_HoldInteractionHandler`))))

(event `self.InteractableArea.OnComponentEndOverlap`
  (params (OverlappedComponent :type "PrimitiveComponent Object Reference") (OtherActor :type "Actor Object Reference") (OtherComp :type "PrimitiveComponent Object Reference") (OtherBodyIndex :type Integer))
  (bind _asbp_base_player (cast `/Game/Blueprints/Core/BP_BasePlayer` OtherActor))
  (`KismetArrayLibrary.Array_RemoveItem` (`self.InteractableActors`) _asbp_base_player)
  (goto _label_2))

(fn `AddRightOffset`
  (params (RightOffset :type "Vector Structure"))
  (set `self.RightOffset` RightOffset)
  (`self.UpdateLocation`)
  (return))

(fn `AddUpOffset`
  (params (UpOffset :type "Vector Structure"))
  (set `self.UpOffset` UpOffset)
  (`self.UpdateLocation`)
  (return))

(fn `UserConstructionScript`)