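; Crane game lever that players hold to pitch it and send a vertical offset to the linked crane.
; A hold interaction handler with no limit drives both lever rotation and crane offset from the current hold seconds.
; The crane's hit-detection event toggles the handler's stop-fires flag each tick.
; Overlapping players are tracked, and whether the first is Anna sets the interaction widget and handler's social type.
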(event `self.ReceiveBeginPlay`
  (bind _bp_holdinteractionhandler (`self.BP_HoldInteractionHandler`))
  (bind _cran (`self.Cran`))
  (`parent.ReceiveBeginPlay`)
  (`|ExecutionSequence`
    (:`then_0`
      (`/Engine/EditorBlueprintResources/StandardMacros.IsValid` _bp_holdinteractionhandler
        (:`Is Valid`
          (set `/Game/Blueprints/Interaction/ActionHandlers/BP_HoldInteractionHandler.bLimited` false _bp_holdinteractionhandler)
          (set `self.InitialRotation` (`SceneComponent.K2_GetComponentRotation` (`self.Lever`)))
          (`/Engine/EditorBlueprintResources/StandardMacros.IsValid` _cran
            (:`Is Valid`
              (set `self.CranInitialLocation` (`SceneComponent.K2_GetComponentLocation` (`Actor.RootComponent` _cran)))
              (add `/Game/Blueprints/Games/Cran/BP_Cran.OnHitDetected` _cran (delegate `OnHitDetected_Event`)))))))
    (:`then_1`
      (add `/Game/Blueprints/Interaction/ActionHandlers/BP_HoldInteractionHandler.HoldUpdated` (`self.BP_HoldInteractionHandler`) (delegate `HoldUpdated_Event`)))))

(event `OnHitDetected_Event`
  (params (BlockingHit :type Boolean))
  (set `self.bHitDetected` BlockingHit))

(event `HoldUpdated_Event`
  (bind _cran (`self.Cran`))
  (`SceneComponent.K2_SetRelativeRotation` (`self.Lever`) (`KismetMathLibrary.ComposeRotators` (`self.InitialRotation`) (`KismetMathLibrary.MakeRotator` 0.0 (* (`/Game/Blueprints/Interaction/ActionHandlers/BP_HoldInteractionHandler.CurrentHoldSeconds` (`self.BP_HoldInteractionHandler`)) 10.0))) false false)
  (`/Engine/EditorBlueprintResources/StandardMacros.IsValid` _cran
    (:`Is Valid`
      (`/Game/Blueprints/Games/Cran/BP_Cran.AddUpOffset` _cran (+ (0.0 0.0 0.0) (`KismetMathLibrary.MakeVector` 0.0 0.0 (* (`/Game/Blueprints/Interaction/ActionHandlers/BP_HoldInteractionHandler.CurrentHoldSeconds` (`self.BP_HoldInteractionHandler`)) 10.0)))))))

(event `self.ReceiveTick`
  (params (DeltaSeconds :type "Float (single-precision)"))
  (`parent.ReceiveTick` DeltaSeconds)
  (`|ExecutionSequence`
    (:`then_0`
      (if (and (not (`self.bHitDetected`)) (`self.bHoldNow`))
        (set `/Game/Blueprints/Interaction/ActionHandlers/BP_HoldInteractionHandler.bShouldStopFires` false (`self.BP_HoldInteractionHandler`) :!label _label)))
    (:`then_1`
      (if (and (`self.bHitDetected`) (`self.bHoldNow`))
        (set `/Game/Blueprints/Interaction/ActionHandlers/BP_HoldInteractionHandler.bShouldStopFires` true (`self.BP_HoldInteractionHandler`) :!label _label_2)))
    (:`then_2`
      (if (and (`self.bHitDetected`) (not (`self.bHoldNow`)))
        (goto _label_2)))
    (:`then_3`
      (if (and (not (`self.bHitDetected`)) (not (`self.bHoldNow`)))
        (goto _label)))))

(event `/Game/Blueprints/Interaction/BPI_Interactable.HoldInteract`
  (params (InvistigaterCharacter :type "/Game/Blueprints/Core/BP_BasePlayer Object Reference"))
  (`self.CheckCanInteract`)
  (if (`self.bCanInteract`)
    (`/Game/Blueprints/Interaction/ActionHandlers/BP_HoldInteractionHandler.Hold` (`self.BP_HoldInteractionHandler`) InvistigaterCharacter)
    (set `self.bHoldNow` true)
    (set `self.bStopCheckDetected` false)
    (`KismetSystemLibrary.RetriggerableDelay` 0.001)
    (set `self.bHoldNow` false)
    (set `self.bStopCheckDetected` true)))

(event `self.InteractableArea.OnComponentBeginOverlap`
  (params (OverlappedComponent :type "PrimitiveComponent Object Reference") (OtherActor :type "Actor Object Reference") (OtherComp :type "PrimitiveComponent Object Reference") (OtherBodyIndex :type Integer) (bFromSweep :type Boolean) (SweepResult :type "HitResult Structure (by ref)"))
  (bind (_actorinteractioninfo_interactiontype _actorinteractioninfo_interactionsocialtype) (break `/Game/Blueprints/Interaction/S_ObjectInteractionInfo` (`self.ActorInteractionInfo`)))
  (bind _asbp_base_player (cast `/Game/Blueprints/Core/BP_BasePlayer` OtherActor))
  (`KismetArrayLibrary.Array_AddUnique` (`self.InteractableActors`) _asbp_base_player)
  (if (>= (`KismetArrayLibrary.Array_Length` (`self.InteractableActors`)) 1) :!label _label_3
    (cast `/Game/Blueprints/Core/BP_Anna` (`|GetArrayItem` (`self.InteractableActors`))
      (:`then`
        (set `self.ActorInteractionInfo` (make `/Game/Blueprints/Interaction/S_ObjectInteractionInfo` "NewEnumerator1")))
      (:`CastFailed`
        (set `self.ActorInteractionInfo` (make `/Game/Blueprints/Interaction/S_ObjectInteractionInfo` "NewEnumerator1" "NewEnumerator1"))))
    (bind _asbpw_interaction_type_widget (cast `/Game/Blueprints/Widgets/Actors/BPW_InteractionTypeWidget` (`WidgetComponent.GetWidget` (`self.Widget`))))
    (`/Game/Blueprints/Widgets/Actors/BPW_InteractionTypeWidget.SetType` _asbpw_interaction_type_widget _actorinteractioninfo_interactiontype _actorinteractioninfo_interactionsocialtype)
    (set `/Game/Blueprints/Interaction/ActionHandlers/BP_HoldInteractionHandler.InteractionSocialType` _actorinteractioninfo_interactionsocialtype (`self.BP_HoldInteractionHandler`))))

(event `self.InteractableArea.OnComponentEndOverlap`
  (params (OverlappedComponent :type "PrimitiveComponent Object Reference") (OtherActor :type "Actor Object Reference") (OtherComp :type "PrimitiveComponent Object Reference") (OtherBodyIndex :type Integer))
  (bind _asbp_base_player (cast `/Game/Blueprints/Core/BP_BasePlayer` OtherActor))
  (`KismetArrayLibrary.Array_RemoveItem` (`self.InteractableActors`) _asbp_base_player)
  (goto _label_3))

(fn `UserConstructionScript`
  (`parent.UserConstructionScript`))