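; Snowman minigame manager that tracks the building of a snowman from snowballs and fires SnowmanCompleted when all are placed, with Anna prompting for the carrot.
; It binds each snowball's events to toggle a tip plane and play color and audio feedback.
; Snowballs are reordered as they reach full shape, shrinking the target size for following ones.
; MoveSnowAlongSpline slides them in that order along big, middle and small splines by progress percent.
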(event `SnowUpdated_Event`
  (for (_array_element _array_index) (`self.Snows`)
    (`KismetArrayLibrary.Array_Insert` (`self.bShouldShowTip`) (and (`/Game/Blueprints/Games/Snowman/BP_Snow.bSnowHasMaxShape` _array_element) (not (`/Game/Blueprints/Games/Snowman/BP_Snow.bSnowPartOfSnowMan` _array_element))) _array_index))
  (if (not (`KismetArrayLibrary.Array_Contains` (`self.bShouldShowTip`) true))
    (`SceneComponent.SetVisibility` (`self.TipPlane`) false false)
    (else
      (`SceneComponent.SetVisibility` (`self.TipPlane`) true false))))

(event `SnowMaxShapeCompleted_Event`
  (params (SnowCompleted :type "/Game/Blueprints/Games/Snowman/BP_Snow Object Reference"))
  (`self.SwapElement` SnowCompleted)
  (`SceneComponent.SetVisibility` (`self.TipPlane`) true false)
  (switch `int` (`self.SnowCount`)
    (:`0`
      (set `self.CurrentSnowSize` 2.2))
    (:`1`
      (set `self.CurrentSnowSize` 1.5)))
  (for _array_element (`self.Snows`)
    (set `/Game/Blueprints/Interaction/ActionHandlers/BP_HoldProgressHandler.HoldDestinationProgress` (`self.CurrentSnowSize`) (`/Game/Blueprints/Games/Snowman/BP_Snow.BP_HoldProgressHandler` _array_element)))
  (`/Engine/EditorBlueprintResources/StandardMacros.IncrementInt` (`self.SnowCount`)))

(event `self.ReceiveBeginPlay`
  (bind _returnvalue (`PrimitiveComponent.CreateDynamicMaterialInstance` (`self.TipPlane`) 0 "/Game/Materials/Additionals/Shaders/MI_ShowBallTIp.MI_ShowBallTIp" "None"))
  (`PrimitiveComponent.SetMaterial` (`self.TipPlane`) 0 _returnvalue)
  (`SceneComponent.SetVisibility` (`self.TipPlane`) false false)
  (for _array_element (`self.Snows`)
    (`/Engine/EditorBlueprintResources/StandardMacros.IsValid` _array_element
      (:`Is Valid`
        (set `/Game/Blueprints/Interaction/ActionHandlers/BP_HoldProgressHandler.HoldDestinationProgress` (`self.CurrentSnowSize`) (`/Game/Blueprints/Games/Snowman/BP_Snow.BP_HoldProgressHandler` _array_element))
        (add `/Game/Blueprints/Games/Snowman/BP_Snow.SnowCompleted` _array_element (delegate `SnowCompleted_Event`))
        (set `/Game/Blueprints/Games/Snowman/BP_Snow.SnowmanGame` self _array_element)
        (add `/Game/Blueprints/Games/Snowman/BP_Snow.SnowMaxShapeCompleted` _array_element (delegate `SnowMaxShapeCompleted_Event`))
        (add `/Game/Blueprints/Games/Snowman/BP_Snow.SnowUpdated` _array_element (delegate `SnowUpdated_Event`))))))

(event `SnowCompleted_Event`
  (`|ExecutionSequence`
    (:`then_0`
      (for (_array_element _array_index) (`self.Snows`)
        (bind _bsnowpartofsnowman (`/Game/Blueprints/Games/Snowman/BP_Snow.bSnowPartOfSnowMan` _array_element))
        (`KismetArrayLibrary.Array_Insert` (`self.bShouldShowTip`) (and (`/Game/Blueprints/Games/Snowman/BP_Snow.bSnowHasMaxShape` _array_element) (not _bsnowpartofsnowman)) _array_index)
        (if _bsnowpartofsnowman
          (set `self.bSnowanHasAllParts` true)
          (else
            (set `self.bSnowanHasAllParts` false)
            (break))))
      (`|ExecutionSequence`
        (:`then_0`
          (if (`self.bSnowanHasAllParts`)
            (`self.SnowmanCompleted`)
            (bind _asbp_two_characters_controller (cast `/Game/Blueprints/Core/BP_TwoCharactersController` (`GameplayStatics.GetPlayerController` 0)))
            (`/Game/Blueprints/Core/BP_BasePlayer.ShowReaction` (`/Game/Blueprints/Core/BP_TwoCharactersController.Anna` _asbp_two_characters_controller) "The last part remains - the carrot!")
            (`SceneComponent.SetVisibility` (`self.TipPlane`) false false)
            (elif (not (`KismetArrayLibrary.Array_Contains` (`self.bShouldShowTip`) true))
              (`SceneComponent.SetVisibility` (`self.TipPlane`) true false)
              (else
                (`SceneComponent.SetVisibility` (`self.TipPlane`) false false)))))
        (:`then_1`
          (bind _asmaterial_instance_dynamic (cast `MaterialInstanceDynamic` (`PrimitiveComponent.GetMaterial` (`self.TipPlane`) 0)))
          (bind (_direction _start) (`Timeline|ColorChange` :`NewTime` 1.0)
            (:`Update`
              (`MaterialInstanceDynamic.SetVectorParameterValue` _asmaterial_instance_dynamic "Color" _start))))))
    (:`then_1`
      (`AudioComponent.Play` (`self.Audio`) 0.0))))

(fn `IsNowRightSnow`
  (params (Snow :type "/Game/Blueprints/Games/Snowman/BP_Snow Object Reference"))
  (returns (Result :type Boolean))
  (return (== (`KismetArrayLibrary.Array_Find` (`self.Snows`) Snow) (`self.SnowToSet`))))

(fn `IsSomeSnowOnAnnaPlace`
  (returns (AnnaPlaceHasSnow :type Boolean))
  (for _array_element (`self.Snows`)
    (if (== (`SceneComponent.K2_GetComponentLocation` (`/Game/Blueprints/Interaction/BP_InteractableActor.StaticMesh` _array_element)) (`SceneComponent.K2_GetComponentLocation` (`self.AnnaPlace`)) :`ErrorTolerance` 5.0)
      (return true)))
  (return false))

(fn `MoveSnowAlongSpline`
  (params (Snow :type "/Game/Blueprints/Games/Snowman/BP_Snow Object Reference"))
  (locals (Distance :type "Float (double-precision)"))
  (bind _returnvalue (`KismetArrayLibrary.Array_Find` (`self.Snows`) Snow))
  (bind _output (`|GetArrayItem` (`self.Snows`) _returnvalue))
  (if (!= _returnvalue -1)
    (if (`/Game/Blueprints/Games/Snowman/BP_Snow.bSnowReadySet` _output)
      (switch `int` _returnvalue
        (:`0`
          (if (== (`self.SnowToSet`) _returnvalue)
            (bind _percent (`/Game/Blueprints/Games/Snowman/BP_Snow.GetProgressPercent` _output))
            (bind _output_get (set `local.Distance` (* _percent (`SplineComponent.GetSplineLength` (`self.BigSnowSpline`)))))
            (`SceneComponent.K2_SetWorldLocation` (`/Game/Blueprints/Interaction/BP_InteractableActor.StaticMesh` _output) (`SplineComponent.GetLocationAtDistanceAlongSpline` (`self.BigSnowSpline`) _output_get "World") false false)
            (if (`/Game/Blueprints/Games/Snowman/BP_Snow.bSnowPartOfSnowMan` _output)
              (set `self.SnowToSet` 1))))
        (:`1`
          (if (== (`self.SnowToSet`) _returnvalue)
            (bind _percent_2 (`/Game/Blueprints/Games/Snowman/BP_Snow.GetProgressPercent` _output))
            (bind _output_get_2 (set `local.Distance` (* _percent_2 (`SplineComponent.GetSplineLength` (`self.MiddleSnowSpline`)))))
            (`SceneComponent.K2_SetWorldLocation` (`/Game/Blueprints/Interaction/BP_InteractableActor.StaticMesh` _output) (`SplineComponent.GetLocationAtDistanceAlongSpline` (`self.MiddleSnowSpline`) _output_get_2 "World") false false)
            (if (`/Game/Blueprints/Games/Snowman/BP_Snow.bSnowPartOfSnowMan` _output)
              (set `self.SnowToSet` 2))))
        (:`2`
          (if (== (`self.SnowToSet`) _returnvalue)
            (bind _percent_3 (`/Game/Blueprints/Games/Snowman/BP_Snow.GetProgressPercent` _output))
            (bind _output_get_3 (set `local.Distance` (* _percent_3 (`SplineComponent.GetSplineLength` (`self.SmallSnowSpline`)))))
            (`SceneComponent.K2_SetWorldLocation` (`/Game/Blueprints/Interaction/BP_InteractableActor.StaticMesh` _output) (`SplineComponent.GetLocationAtDistanceAlongSpline` (`self.SmallSnowSpline`) _output_get_3 "World") false false)
            (if (`/Game/Blueprints/Games/Snowman/BP_Snow.bSnowPartOfSnowMan` _output)
              (set `self.SnowToSet` -1))))))))

(fn `SwapElement`
  (params (SnowToSwap :type "/Game/Blueprints/Games/Snowman/BP_Snow Object Reference"))
  (locals (TempSnow :type "/Game/Blueprints/Games/Snowman/BP_Snow Object Reference"))
  (bind _snows (`self.Snows`))
  (bind _snowcount (`self.SnowCount`))
  (bind _output_get (set `local.TempSnow` SnowToSwap))
  (bind _returnvalue (`KismetArrayLibrary.Array_Find` (`self.Snows`) _output_get))
  (if (== _returnvalue _snowcount)
    (return)
    (else
      (`KismetArrayLibrary.Array_Set` _snows _returnvalue (`|GetArrayItem` _snows _snowcount))
      (`KismetArrayLibrary.Array_Set` _snows _snowcount (`local.TempSnow`))
      (return))))

(fn `UserConstructionScript`)