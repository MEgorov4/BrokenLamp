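; Two-player co-op bookcase that Anna and Leon topple by holding interact together.
; HoldInteract keeps BothInteract alive with a tiny retriggerable delay, letting Tick tilt the mesh, or ease it back upright on release.
; Near -45° roll it fires OnStartFalling, which restarts the game timer, plays the fall timeline with audio and marks completion.
; Players inside TipBox block tilting and show a warning reaction when both interact.
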(event `self.ReceiveBeginPlay`
  (`parent.ReceiveBeginPlay`)
  (add `self.OnStartFalling` (`|CreateDelegate` :!event `OnStartFalling_Event`)))

(event `OnStartFalling_Event`
  (bind (_returnvalue_roll _returnvalue_pitch _returnvalue_yaw) (`KismetMathLibrary.BreakRotator` (`SceneComponent.K2_GetComponentRotation` (`self.StaticMesh`))))
  (bind _asbp_two_players_game_instance (cast `/Game/Blueprints/Core/BP_TwoPlayersGameInstance` (`GameplayStatics.GetGameInstance`)))
  (`/Game/Blueprints/Core/BP_TwoPlayersGameInstance.StopTimer` _asbp_two_players_game_instance)
  (`/Game/Blueprints/Core/BP_TwoPlayersGameInstance.StartTimer` _asbp_two_players_game_instance 300.0)
  (`|ExecutionSequence`
    (:`then_0`
      (bind (_direction _valur) (`Timeline|BookcaseFalling`)
        (:`Update`
          (`SceneComponent.K2_SetWorldRotation` (`self.StaticMesh`) (`KismetMathLibrary.MakeRotator` _valur _returnvalue_pitch _returnvalue_yaw) false false))
        (:`EventTrack`
          (`AudioComponent.Play` (`self.Audio`) 0.0))))
    (:`then_1`
      (set `self.bCompleted` true))))

(event `self.ReceiveTick`
  (params (DeltaSeconds :type "Float (single-precision)"))
  (bind _bshouldinteract (`self.bShouldInteract`))
  (bind _returnvalue_roll (`KismetMathLibrary.BreakRotator` (`SceneComponent.K2_GetComponentRotation` (`self.StaticMesh`))))
  (bind _returnvalue_roll_2 (`KismetMathLibrary.BreakRotator` (`SceneComponent.K2_GetComponentRotation` (`self.StaticMesh`))))
  (`parent.ReceiveTick` DeltaSeconds)
  (if (== (`KismetArrayLibrary.Array_Length` (`self.TipBoxChecker`)) 0)
    (if (and (`self.bBothInteract`) _bshouldinteract)
      (`SceneComponent.K2_AddRelativeRotation` (`self.StaticMesh`) (`KismetMathLibrary.MakeRotator` (* DeltaSeconds -1.0 25.0)) true false)
      (if (`KismetMathLibrary.NearlyEqual_FloatFloat` _returnvalue_roll -45.0 1.0)
        (set `self.bShouldInteract` false)
        (`self.OnStartFalling`))
      (elif (and _bshouldinteract (not (`KismetMathLibrary.NearlyEqual_FloatFloat` _returnvalue_roll_2 0.0 1.0)))
        (`SceneComponent.K2_AddRelativeRotation` (`self.StaticMesh`) (`KismetMathLibrary.MakeRotator` (* DeltaSeconds 1.0 25.0)) true false)))
    (elif (`self.bBothInteract`)
      (`/Game/Blueprints/Core/BP_BasePlayer.ShowReaction` (`|GetArrayItem` (`self.TipBoxChecker`)) "Не стоит стоять под шкафом..."))))

(event `/Game/Blueprints/Interaction/BPI_Interactable.HoldInteract`
  (params (InvistigaterCharacter :type "/Game/Blueprints/Core/BP_BasePlayer Object Reference"))
  (bind _asbp_two_characters_controller (cast `/Game/Blueprints/Core/BP_TwoCharactersController` (`GameplayStatics.GetPlayerController` 0)))
  (bind _return (`self.CheckCanInteract`))
  (if (and _return (`/Game/Blueprints/Core/BP_TwoCharactersController.AnnaHoldInteract` _asbp_two_characters_controller) (`/Game/Blueprints/Core/BP_TwoCharactersController.LeonHoldInteract` _asbp_two_characters_controller))
    (`KismetSystemLibrary.PrintString` "Bookcase" true true (struct :`G` 0.66 :`B` 1.0 :`A` 1.0) 0.0)
    (set `self.bBothInteract` true)
    (`KismetSystemLibrary.RetriggerableDelay` 0.001)
    (set `self.bBothInteract` false)))

(event `self.TipBox.OnComponentBeginOverlap`
  (params (OverlappedComponent :type "PrimitiveComponent Object Reference") (OtherActor :type "Actor Object Reference") (OtherComp :type "PrimitiveComponent Object Reference") (OtherBodyIndex :type Integer) (bFromSweep :type Boolean) (SweepResult :type "HitResult Structure (by ref)"))
  (bind _asbp_base_player (cast `/Game/Blueprints/Core/BP_BasePlayer` OtherActor))
  (`KismetArrayLibrary.Array_AddUnique` (`self.TipBoxChecker`) _asbp_base_player))

(event `self.TipBox.OnComponentHit`
  (params (HitComponent :type "PrimitiveComponent Object Reference") (OtherActor :type "Actor Object Reference") (OtherComp :type "PrimitiveComponent Object Reference") (NormalImpulse :type "Vector Structure") (Hit :type "HitResult Structure (by ref)")))

(event `self.TipBox.OnComponentEndOverlap`
  (params (OverlappedComponent :type "PrimitiveComponent Object Reference") (OtherActor :type "Actor Object Reference") (OtherComp :type "PrimitiveComponent Object Reference") (OtherBodyIndex :type Integer))
  (bind _asbp_base_player (cast `/Game/Blueprints/Core/BP_BasePlayer` OtherActor))
  (`KismetArrayLibrary.Array_RemoveItem` (`self.TipBoxChecker`) _asbp_base_player))

(fn `UserConstructionScript`
  (`parent.UserConstructionScript`))