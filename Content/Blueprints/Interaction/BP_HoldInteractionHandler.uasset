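; Hold-to-interact handler for an owning BP_InteractableActor, supporting interactions held by Anna, Leon or both together.
; Repeated Hold calls keep each character's flag raised through a very short retriggerable delay.
; Tick feeds a gate that raises or decays the hold progress according to the owner's social type and those flags.
; Nearing the target duration fires HoldCompleted once and closes the gate, which Refresh opens.
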(event `self.ReceiveBeginPlay`
  (bind _asbp_interactable_actor (cast `/Game/Blueprints/Interaction/BP_InteractableActor` (`self.GetOwner`)))
  (bind (_actorinteractioninfo_interactiontype _actorinteractioninfo_interactionsocialtype) (break `/Game/Blueprints/Interaction/S_ObjectInteractionInfo` (`/Game/Blueprints/Interaction/BP_InteractableActor.ActorInteractionInfo` _asbp_interactable_actor)))
  (set `self.InteractionSocialType` _actorinteractioninfo_interactionsocialtype))

(event `Refresh`
  (goto _label :!via `Open`))

(event `self.ReceiveTick`
  (params (DeltaSeconds :type "Float (single-precision)"))
  (`|ExecutionSequence`
    (:`then_0`
      (`/Engine/EditorBlueprintResources/StandardMacros.Gate` false :!label _label
        (:`Exit`
          (switch `/Game/Blueprints/Interaction/E_InteractionSocialType` (`self.InteractionSocialType`)
            (:`NewEnumerator0`
              (if (`self.AnnaHold`)
                (`self.HoldScoreAdd` (`self.HoldAddSpeed`) :!label _label_2)
                (else
                  (`self.HoldScoreFires` (`self.HoldFiresSpeed`) :!label _label_3))))
            (:`NewEnumerator1`
              (if (`self.LeonHold`)
                (goto _label_2)
                (else
                  (goto _label_3))))
            (:`NewEnumerator2`
              (if (and (`self.LeonHold`) (`self.AnnaHold`))
                (goto _label_2)
                (else
                  (goto _label_3))))))))
    (:`then_1`
      (if (`KismetMathLibrary.NearlyEqual_FloatFloat` (`self.HoldDestinationSeconds`) (`self.CurrentHoldSeconds`) 0.1)
        (`/Engine/EditorBlueprintResources/StandardMacros.DoOnce` false
          (:`Completed`
            (`self.HoldCompleted`)
            (goto _label :!via `Close`)))))
    (:`then_2`
      (`KismetSystemLibrary.PrintString` (`KismetStringLibrary.Conv_DoubleToString` (`self.CurrentHoldSeconds`)) true true (struct :`G` 0.66 :`B` 1.0 :`A` 1.0) 0.0))))

(event `Hold`
  (params (Invistigator :type "/Game/Blueprints/Core/BP_BasePlayer Object Reference"))
  (if (`GameplayStatics.ObjectIsA` Invistigator "/Game/Blueprints/Core/BP_Leon.BP_Leon_C")
    (set `self.LeonHold` true)
    (`KismetSystemLibrary.RetriggerableDelay` 0.001)
    (set `self.LeonHold` false)
    (else
      (set `self.AnnaHold` true)
      (`KismetSystemLibrary.RetriggerableDelay` 0.001)
      (set `self.AnnaHold` false))))