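; BP_BothGoToLevel is an interactable that fires a level-travel completion only while two players stand in its area.
; InteractableArea overlaps add and remove BP_BasePlayer actors in TipBoxChecker.
; PressInteract requires exactly two entries, prints a leftover debug string, then calls PressCompleted0 with GoToLevel if CheckCanInteract passes.
; The level change itself is handled outside these graphs.
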(event `self.ReceiveBeginPlay`
  (`parent.ReceiveBeginPlay`))

(event `self.PressInteract`
  (params (InvistigaterCharacter :type "/Game/Blueprints/Core/BP_BasePlayer Object Reference"))
  (if (== (`KismetArrayLibrary.Array_Length` (`self.TipBoxChecker`)) 2)
    (`KismetSystemLibrary.PrintString` "bitch")
    (bind _return (`self.CheckCanInteract`))
    (if _return
      (`self.PressCompleted_0` (`self.GoToLevel`)))))

(event `self.InteractableArea.OnComponentBeginOverlap`
  (params (OverlappedComponent :type "PrimitiveComponent Object Reference") (OtherActor :type "Actor Object Reference") (OtherComp :type "PrimitiveComponent Object Reference") (OtherBodyIndex :type Integer) (bFromSweep :type Boolean) (SweepResult :type "HitResult Structure (by ref)"))
  (bind _asbp_base_player (cast `/Game/Blueprints/Core/BP_BasePlayer` OtherActor))
  (`KismetArrayLibrary.Array_AddUnique` (`self.TipBoxChecker`) _asbp_base_player))

(event `self.InteractableArea.OnComponentEndOverlap`
  (params (OverlappedComponent :type "PrimitiveComponent Object Reference") (OtherActor :type "Actor Object Reference") (OtherComp :type "PrimitiveComponent Object Reference") (OtherBodyIndex :type Integer))
  (bind _asbp_base_player (cast `/Game/Blueprints/Core/BP_BasePlayer` OtherActor))
  (`KismetArrayLibrary.Array_RemoveItem` (`self.TipBoxChecker`) _asbp_base_player))

(fn `UserConstructionScript`
  (`parent.UserConstructionScript`))