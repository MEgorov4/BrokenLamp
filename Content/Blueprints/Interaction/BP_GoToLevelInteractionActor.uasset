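; BP_GoToLevelInteractionActor is an interactable actor that, going by its name and payload, requests a level change.
; On PressInteract it prints a leftover debug string, runs CheckCanInteract, and, if CanInteract is true, calls PressCompleted0 with GoToLevel.
; The level load itself is not handled in this graph.
; BeginPlay and the construction script only call the parent, while Tick and overlap events are disabled.
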(event `self.ReceiveBeginPlay`
  (`parent.ReceiveBeginPlay`))

(event `/Game/Blueprints/Interaction/BPI_Interactable.PressInteract`
  (params (InvistigaterCharacter :type "/Game/Blueprints/Core/BP_BasePlayer Object Reference"))
  (`KismetSystemLibrary.PrintString` "bitch")
  (`self.CheckCanInteract`)
  (if (`self.bCanInteract`)
    (`self.PressCompleted_0` (`self.GoToLevel`))))

(fn `UserConstructionScript`
  (`parent.UserConstructionScript`))